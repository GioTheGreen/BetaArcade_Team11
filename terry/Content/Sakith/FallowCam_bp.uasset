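; Shared follow camera that keeps all active players in view once GameStarted hands it the player list.
; Each tick it lerps its center point toward the players' average location.
; It then sets the spring arm length to the largest pairwise distance between players, clamped to a minimum and maximum.
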(event `self.ReceiveTick`
  (params (DeltaSeconds :type "Float (single-precision)"))
  (if (`self.IsGameStarted`)
    (`self.Calculate Cam Movement`)
    (`self.Calculate Cam Zoom`)))

(fn `Calculate Cam Movement`
  (set `self.Loacation-` (`SceneComponent.K2_GetComponentLocation` (`self.CenterPoint`)))
  (bind _returnvalue (`GameplayStatics.GetActorArrayAverageLocation` (`self.Active Players`)))
  (`SceneComponent.K2_SetWorldLocation` (`self.CenterPoint`) (`KismetMathLibrary.VLerp` (`self.Loacation-`) _returnvalue (`self.CamLerpSpeed`)) false false))

(fn `Calculate Cam Zoom`
  (bind _active_players (`self.Active Players`))
  (for (_array_element _array_index) _active_players
    (set `self.Current Player` _array_element)
    (for _index (range (+ _array_index 1) (`KismetArrayLibrary.Array_Length` _active_players))
      (`KismetArrayLibrary.Array_Add` (`self.Distence`) (`self.GetDistanceTo` (`self.Current Player`) (`|GetArrayItem` (`self.Active Players`) _index)))))
  (set `SpringArmComponent.TargetArmLength` (`KismetMathLibrary.FClamp` (`.MaxValue` (`KismetMathLibrary.MaxOfFloatArray` (`self.Distence`))) (`self.MinSpringArmLength`) (`self.MaxSpringArmLength`)) (`self.SpringArm`))
  (`KismetArrayLibrary.Array_Clear` (`self.Distence`)))

(fn `GameStarted`
  (params (ActivePlayers :type "Array of /Game/Sakith/SakithsPlayer_bp Object Reference"))
  (set `self.Active Players` ActivePlayers)
  (set `self.IsGameStarted` true))

(fn `UserConstructionScript`)
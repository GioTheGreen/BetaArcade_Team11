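; Local multiplayer manager that adds a UI widget and sets up local players at the level's PlayerStarts on BeginPlay.
; It matches numeric PlayerStart tags to indices, creating a local player and spawning a possessed InputReciver_bp for each match, tracking receivers and controllers in arrays.
; SpwanPlayer later spawns a SakithsPlayer_bp at a given receiver's transform and hands that player's controller over to it.
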(event `self.ReceiveBeginPlay`
  ;[0.2908 0.702 1] Safty check
  (bind _returnvalue (`|CreateWidget` "/Game/Sakith/Sakiths_wdt.Sakiths_wdt_C"))
  (`UserWidget.AddToViewport` _returnvalue 0)
  ;[1 1 1] Player Locations
  (`self.GetPlayerStartPoints`)
  (`self.SpwanInputRecivers`))

(fn `GetPlayerStartPoints`
  (bind _outactors (`GameplayStatics.GetAllActorsOfClass` "/Script/Engine.PlayerStart"))
  (set `self.PlayerStartArray` _outactors))

(fn `SpwanInputRecivers`
  (locals (Index :type Integer))
  (for (_ _array_index) (`self.PlayerStartArray`)
    (set `local.Index` _array_index)
    (for (_array_element _array_index_2) (`self.PlayerStartArray`)
      (if (== (`KismetStringLibrary.Conv_StringToInt` (`KismetStringLibrary.Conv_NameToString` (`PlayerStart.PlayerStartTag` _array_element))) (`local.Index`))
        (`GameplayStatics.CreatePlayer` -1)
        (bind _returnvalue (`|SpawnActorFromClass` "/Game/Sakith/InputReciver_bp.InputReciver_bp_C" (`self.GetTransform` _array_element) "Undefined" "OverrideRootScale" null _array_index_2 null))
        (`KismetArrayLibrary.Array_AddUnique` (`self.InputRecivers`) _returnvalue)
        (bind _returnvalue_2 (`GameplayStatics.GetPlayerController` _array_index_2))
        (`Controller.Possess` _returnvalue_2 _returnvalue)
        (`KismetArrayLibrary.Array_AddUnique` (`self.PlayerControllers`) _returnvalue_2)))))

(fn `SpwanPlayer`
  (params (PlayerIndex :type Integer) (InputReciver :type "/Game/Sakith/InputReciver_bp Object Reference"))
  (returns (Return0 :type Boolean))
  (bind _returnvalue (`|SpawnActorFromClass` "/Game/Sakith/SakithsPlayer_bp.SakithsPlayer_bp_C" (`self.GetTransform` (`local.InputReciver`)) "Undefined" "OverrideRootScale" null (`local.PlayerIndex`) null))
  (`Controller.Possess` (`GameplayStatics.GetPlayerController` (`local.PlayerIndex`)) _returnvalue)
  (return false))

(fn `UserConstructionScript`)
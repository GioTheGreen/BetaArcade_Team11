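; Sword-swing projectile actor that knocks back players it overlaps, sparing the character held in its Ignore variable.
; When the Box begins overlapping another SakithsPlayer_bp, it launches that player horizontally away from the Ignore character's capsule, with a fixed upward boost.
; The push direction comes from the Ignore character's position rather than the projectile's, and no damage is applied here.
; The construction script sets the actor's life span from the Lifespan variable.
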(event `self.Box.OnComponentBeginOverlap`
  (params (OverlappedComponent :type "PrimitiveComponent Object Reference") (OtherActor :type "Actor Object Reference") (OtherComp :type "PrimitiveComponent Object Reference") (OtherBodyIndex :type Integer) (bFromSweep :type Boolean) (SweepResult :type "HitResult Structure (by ref)"))
  (bind _ignore (`self.ignore`))
  (bind _assakiths_player_bp (cast `/Game/Sakith/SakithsPlayer_bp` OtherActor))
  (if (!= _assakiths_player_bp _ignore)
    (bind (_returnvalue_x _returnvalue_y) (`KismetMathLibrary.BreakVector` (* (`KismetMathLibrary.Normal` (- (`SceneComponent.K2_GetComponentLocation` (`Character.CapsuleComponent` _assakiths_player_bp)) (`SceneComponent.K2_GetComponentLocation` (`Character.CapsuleComponent` _ignore)))) 500.0)))
    (`Character.LaunchCharacter` _assakiths_player_bp (`KismetMathLibrary.MakeVector` _returnvalue_x _returnvalue_y 400.0) false false)))

(fn `UserConstructionScript`
  (`parent.UserConstructionScript`)
  (`self.SetLifeSpan` (`self.lifespan`)))